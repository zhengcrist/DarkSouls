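; BP_Enemy is an enemy with a skeletal mannequin mesh that loses health when attacked and plays a death animation.
; It sets HP on BeginPlay and takes smaller or larger damage from the BPIAttack and BPIHeavyAttack events.
; Both events share one path that prints HP in red and plays a non-looping knockdown death animation at zero or below, without destroying the actor or blocking further hits.
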(event `self.ReceiveBeginPlay`
  (set `self.HP` 20))

(event `/Game/BPI_Attack.BPI_Attack`
  (bind _hp (`self.HP`))
  (set `self.HP` (- _hp 2))
  (`KismetSystemLibrary.PrintString` (`KismetStringLibrary.Conv_IntToString` _hp) true true (struct :`R` 1.0 :`G` 0.060021 :`A` 1.0) :!label _label)
  (if (<= _hp 0)
    (`SkeletalMeshComponent.PlayAnimation` (`self.SK_Mannequin`) "/Game/Sword_Animations/Animations/Sequence1/08_Hit/11_Knock_Down_Combat/Knock_Down_Combat_Death_Seq.Knock_Down_Combat_Death_Seq" false)))

(event `/Game/BPI_HeavyAttack.BPI_HeavyAttack`
  (set `self.HP` (- (`self.HP`) 5))
  (goto _label))

(fn `UserConstructionScript`)