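; Player character Blueprint for third-person-style melee play, handling camera look, movement, sprint, roll and sword attacks through Enhanced Input and raw keys.
; Space sprints by changing walk speed and rotation mode, while a short IA_Roll press during movement plays a roll montage.
; Attacks trace forward, then message the hit actor via interface as the montage starts, with Shift selecting heavy.
; IsAttacking and InAction flags block overlapping actions, and attacking blocks movement.
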(event `self.ReceiveBeginPlay`
  ;[1 0.2083 0.2083] Event begin
  (bind _asplayer_controller (cast `PlayerController` (`self.GetController`)))
  (`EnhancedInputSubsystemInterface.AddMappingContext` (pcsubsystem `EnhancedInputLocalPlayerSubsystem` _asplayer_controller) "/Game/Inputs/IMC_Player.IMC_Player" 0 (struct))
  (set `self.isAttacking` false))

(event `EnhancedInput|/Game/Inputs/Actions/IA_Look`
  (params (ActionValue :type "Vector2D Structure") (ElapsedSeconds :type "Float (double-precision)") (TriggeredSeconds :type "Float (double-precision)") (InputAction :type "InputAction Object Reference" :default "/Game/Inputs/Actions/IA_Look.IA_Look"))
  ;[0.2753 0.7773 1] Look
  (:`Triggered`
    (`self.AddControllerYawInput` ActionValue_X)
    (`self.AddControllerPitchInput` ActionValue_Y)))

(event `EnhancedInput|/Game/Inputs/Actions/IA_Move`
  (params (ActionValue :type "Vector2D Structure") (ElapsedSeconds :type "Float (double-precision)") (TriggeredSeconds :type "Float (double-precision)") (InputAction :type "InputAction Object Reference" :default "/Game/Inputs/Actions/IA_Move.IA_Move"))
  (bind (_returnvalue_roll _returnvalue_pitch _returnvalue_yaw) (`KismetMathLibrary.BreakRotator` (`SceneComponent.K2_GetComponentRotation` (`self.Camera`))))
  ;[0.4567 1 0.4791] Move
  (:`Triggered`
    (if (not (`self.isAttacking`))
      (`self.AddMovementInput` (`KismetMathLibrary.GetForwardVector` (`KismetMathLibrary.MakeRotator` 0.0 0.0 _returnvalue_yaw)) ActionValue_X)
      (`self.AddMovementInput` (`KismetMathLibrary.GetRightVector` (`KismetMathLibrary.MakeRotator` 0.0 0.0 _returnvalue_yaw)) ActionValue_Y)))
  (:`Started`
    (set `self.Move` true))
  (:`Completed`
    (set `self.Move` false)))

(event `Key|SpaceBar`
  (params (Key :type "Key Structure"))
  (bind _charactermovement (`self.CharacterMovement`))
  (bind _charactermovement_2 (`self.CharacterMovement`))
  ;[0.4158 1 0.5126] Sprint
  (:`Pressed`
    (if (`self.Move`)
      (set `CharacterMovementComponent.MaxWalkSpeed` 900.0 _charactermovement_2)
      (set `CharacterMovementComponent.bUseControllerDesiredRotation` false _charactermovement_2)
      (set `CharacterMovementComponent.bOrientRotationToMovement` true _charactermovement_2)))
  (:`Released`
    (set `CharacterMovementComponent.MaxWalkSpeed` 600.0 _charactermovement)
    (set `CharacterMovementComponent.bUseControllerDesiredRotation` true _charactermovement)
    (set `CharacterMovementComponent.bOrientRotationToMovement` false _charactermovement)))

(event `EnhancedInput|/Game/Inputs/Actions/IA_Roll`
  (params (ActionValue :type Boolean) (ElapsedSeconds :type "Float (double-precision)") (TriggeredSeconds :type "Float (double-precision)") (InputAction :type "InputAction Object Reference" :default "/Game/Inputs/Actions/IA_Roll.IA_Roll"))
  ;[0.7966 1 0.4534] Roll
  (:`Completed`
    (if (and (`self.Move`) (not (`self.inAction`)) (< TriggeredSeconds 0.25))
      (set `self.inAction` true)
      (`|PlayMontage` (`self.Mesh`) "/Game/Sword_Animations/Animations/Sequence1/07_Roll/04_Roll_Combat_to_Run/Roll_Combat_to_Run_Fast_Seq_Montage.Roll_Combat_to_Run_Fast_Seq_Montage"
        (:`OnCompleted`
          _)
        (:`OnInterrupted`
          _))
      (set `self.inAction` false))))

(event `EnhancedInput|/Game/Inputs/Actions/IA_Attack`
  (params (ActionValue :type Boolean) (ElapsedSeconds :type "Float (double-precision)") (TriggeredSeconds :type "Float (double-precision)") (InputAction :type "InputAction Object Reference" :default "/Game/Inputs/Actions/IA_Attack.IA_Attack"))
  (bind _capsulecomponent (`self.CapsuleComponent`))
  (bind _mesh (`self.Mesh`))
  (bind _returnvalue (`SceneComponent.K2_GetComponentLocation` _capsulecomponent))
  ;[1 0.6402 0.2425] Attack
  (:`Triggered`
    (if (and (not (`self.isAttacking`)) (not (`self.inAction`)))
      (set `self.isAttacking` true)
      (set `self.inAction` true)
      (bind _outhit (`KismetSystemLibrary.LineTraceSingle` :`Start` _returnvalue :`End` (+ _returnvalue (* (`SceneComponent.GetForwardVector` _capsulecomponent) 300.0)) :`TraceChannel` "TraceTypeQuery1" :`DrawDebugType` "ForDuration"))
      (if (stale `Key|LeftShift` _output_get)
        (`|PlayMontage` _mesh "/Game/Sword_Animations/Animations/Sequence1/02_Attack/03_Combo_Attack_03/Combo_Attack_03_01_Seq_Montage.Combo_Attack_03_01_Seq_Montage"
          (:`then`
            (`GameplayStatics.PlaySoundAtLocation` "/Game/Audio/sword-stab-pull-melee-weapon-236207.sword-stab-pull-melee-weapon-236207" _returnvalue (struct) 1.0 1.0 0.0 null null null null)
            (message `/Game/Player/BPI_HeavyAttack.BPI_HeavyAttack` (`.HitActor` (`GameplayStatics.BreakHitResult` _outhit))))
          (:`OnCompleted`
            (set `self.isAttacking` false :!label _label)
            (set `self.inAction` false))
          (:`OnInterrupted`
            (goto _label)))
        (else
          (`|PlayMontage` _mesh "/Game/Sword_Animations/Animations/Sequence1/02_Attack/03_Combo_Attack_03/Combo_Attack_03_02_Seq_Montage.Combo_Attack_03_02_Seq_Montage"
            (:`then`
              (`GameplayStatics.PlaySoundAtLocation` "/Game/Audio/sword-sound-effect-2-234986.sword-sound-effect-2-234986" _returnvalue (struct) 1.0 1.0 0.0 null null null null)
              (message `/Game/Player/BPI_Attack.BPI_Attack` (`.HitActor` (`GameplayStatics.BreakHitResult` _outhit))))
            (:`OnCompleted`
              (goto _label))
            (:`OnInterrupted`
              (goto _label))))))))

(event `Key|LeftShift`
  (params (Key :type "Key Structure"))
  ;[1 0.6402 0.2425] Attack
  (:`Pressed`
    (bind _output_get (set `self.HeavyAttack` true)))
  (:`Released`
    (set `self.HeavyAttack` false)))

(fn `UserConstructionScript`)