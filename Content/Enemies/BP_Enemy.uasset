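; BP_Enemy is a melee enemy that takes damage, shows a health bar and dies with an animation and sound.
; BPIAttackP subtracts HP and refreshes the widget, which turns toward the player camera every tick.
; While alive and flagged by DoTheAnnoyingThing, overlap turns the mesh toward the actor and replays an attack montage until overlap ends or HP runs out.
; CheckDeath returns true while alive, despite its name.
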(event `HealthRotation`
  (bind _widget (`self.Widget`))
  ;[1 1 1] Health widget
  (`SceneComponent.K2_SetWorldRotation` _widget (`KismetMathLibrary.FindLookAtRotation` (`SceneComponent.K2_GetComponentLocation` _widget) (`SceneComponent.K2_GetComponentLocation` (`Actor.RootComponent` (`GameplayStatics.GetPlayerCameraManager` 0)))) false false))

(event `self.ReceiveBeginPlay`
  ;[1 0.6946 0] cause unreal is a troll
  (`self.SetActorTickEnabled` true)
  (bind _aswg_health_bar (cast `/Game/Enemies/WG_HealthBar` (`WidgetComponent.GetWidget` (`self.Widget`))))
  (set `self.HealthWidget` _aswg_health_bar))

(event `self.ReceiveTick`
  (params (DeltaSeconds :type "Float (single-precision)"))
  (`self.HealthRotation`))

(event `/Game/Player/BPI_AttackP.BPI_AttackP`
  (params (Dmg :type "Float (double-precision)"))
  (bind _hp (`self.HP`))
  ;[1 0.276 0.276] GetHit
  (if (> _hp 0.0)
    (set `self.HP` (- _hp Dmg))
    (`self.UpdateHealth`)
    (bind _notdead (`self.Check Death`))
    (if (not _notdead)
      (`self.Death`))))

(event `Death`
  (set `self.HP` 0.0)
  (`SkeletalMeshComponent.PlayAnimation` (`self.SK_Mannequin`) "/Game/Sword_Animations/Animations/Sequence1/08_Hit/11_Knock_Down_Combat/Knock_Down_Combat_Death_Seq.Knock_Down_Combat_Death_Seq" false)
  (`GameplayStatics.PlaySoundAtLocation` "/Game/Audio/male-death-sound-128357.male-death-sound-128357" (`SceneComponent.K2_GetComponentLocation` (`self.SK_Mannequin`)) (struct) 1.0 1.0 0.0 null null null null))

(event `self.ReceiveActorBeginOverlap`
  (params (OtherActor :type "Actor Object Reference"))
  (bind _sk_mannequin (`self.SK_Mannequin`))
  (bind (_returnvalue_roll _returnvalue_pitch _returnvalue_yaw) (`KismetMathLibrary.BreakRotator` (`KismetMathLibrary.FindLookAtRotation` (`SceneComponent.K2_GetComponentLocation` _sk_mannequin) (`self.K2_GetActorLocation` OtherActor))))
  ;[1 1 1] Attack
  (bind _notdead (`self.Check Death`))
  (if (and _notdead (`self.DoTheAnnoyingThing`))
    (set `self.Colliding` true)
    (`SceneComponent.K2_SetWorldRotation` _sk_mannequin (`KismetMathLibrary.MakeRotator` 0.0 0.0 (+ _returnvalue_yaw -75.0)) false false :!label _label)
    (if (not (`self.Wait`))
      (set `self.Wait` true)
      (`|PlayMontage` (`self.SK_Mannequin`) "/Game/Sword_Animations/Animations/Sequence1/02_Attack/16_Power_Attack/Power_Attack_End_Seq_Montage.Power_Attack_End_Seq_Montage"
        (:`OnCompleted`
          (set `self.Wait` false)
          (bind _notdead_2 (`self.Check Death`))
          (if (and (`self.Colliding`) _notdead_2)
            (goto _label)))))))

(event `self.ReceiveActorEndOverlap`
  (params (OtherActor :type "Actor Object Reference"))
  ;[1 1 1] Attack
  (set `self.Colliding` false))

(fn `Check Death`
  (returns (NotDead :type Boolean))
  (if (> (`self.HP`) 0.0)
    (return true)
    (else
      (return false))))

(fn `UpdateHealth`
  (`/Game/Enemies/WG_HealthBar.RefreshHealth` (`self.HealthWidget`) (`self.HP`)))

(fn `UserConstructionScript`)